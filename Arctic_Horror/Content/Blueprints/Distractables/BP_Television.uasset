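; BP_Television is an interactable distraction object that makes noise at its location when used.
; Its Interact event checks CanPressF and CanInteract, prints a debug message, then reports a noise event with itself as instigator.
; CanInteract is cleared during a 0.2-second delay to throttle repeated triggers.
; The construction script only calls its parent, and the other stock events are empty.
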(event `/Game/Interfaces/BPI_Interactable.Interact`
  (if (`self.CanPressF`)
    (if (`self.CanInteract`)
      (set `self.CanInteract` false)
      (`KismetSystemLibrary.PrintString` "DISTRACTING")
      (`AISense_Hearing.ReportNoiseEvent` (`self.K2_GetActorLocation` self) 1.0 self)
      (`KismetSystemLibrary.Delay` 0.2)
      (set `self.CanInteract` true))))

(fn `UserConstructionScript`
  (`parent.UserConstructionScript`))