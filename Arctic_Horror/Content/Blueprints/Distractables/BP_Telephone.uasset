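; BP_Telephone is a distractable phone that, on interaction, makes a noise to distract the enemy referenced by EnemyBP.
; Interact is gated by CanPressF and CanInteract, with a short delay before it can fire again.
; It briefly switches the enemy AI controller's perception components, turning off the first and activating the others, reports a noise at the phone, then restores the first after a delay.
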(event `/Game/Interfaces/BPI_Interactable.Interact`
  (if (`self.CanPressF`)
    (if (`self.CanInteract`)
      (set `self.CanInteract` false)
      (`KismetSystemLibrary.PrintString` "DISTRACTING")
      (for (_array_element _array_index) (`self.K2_GetComponentsByClass` (`AIBlueprintHelperLibrary.GetAIController` (`self.EnemyBP`)) "/Script/AIModule.AIPerceptionComponent")
        (if (== _array_index 0)
          (`ActorComponent.Deactivate` _array_element)
          (else
            (`ActorComponent.Activate` _array_element true)
            (`AISense_Hearing.ReportNoiseEvent` (`self.K2_GetActorLocation` self) 1.0 self)
            (`KismetSystemLibrary.Delay` 0.2)
            (for (_array_element_2 _array_index_2) (`self.K2_GetComponentsByClass` (`AIBlueprintHelperLibrary.GetAIController` (`self.EnemyBP`)) "/Script/AIModule.AIPerceptionComponent")
              (if (== _array_index_2 0)
                (`ActorComponent.Activate` _array_element_2 true)
                (else
                  (`ActorComponent.Deactivate` _array_element_2)))))))
      (`KismetSystemLibrary.Delay` 0.2)
      (set `self.CanInteract` true))))

(fn `UserConstructionScript`
  (`parent.UserConstructionScript`))