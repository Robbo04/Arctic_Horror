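; Table hiding spot that lets the third-person character toggle hiding when the player presses Interact inside its Detection volume.
; Overlap begin and end switch actor input and open or close a gate on the interact action.
; ToggleHide plays an FMOD sound, calls HidingVignette, toggles character collision, hides the character on entry, and blends the camera between table and player.
; A separate Interact event only runs a cooldown flag.
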(event `self.ReceiveBeginPlay`
  (bind _returnvalue (`GameplayStatics.GetActorOfClass` "/Game/ThirdPerson/Blueprints/BP_ThirdPersonCharacter.BP_ThirdPersonCharacter_C"))
  (set `self.RefThirdPersonCharacter` _returnvalue))

(event `/Game/Interfaces/BPI_Interactable.Interact`
  (if (`self.CanPressF`)
    (if (`self.CanInteract`)
      (set `self.CanInteract` false)
      (`KismetSystemLibrary.Delay` 2.0)
      (set `self.CanInteract` true))))

(event `EnhancedInput|/Game/ThirdPerson/Input/Actions/IA_Interact`
  (params (ActionValue :type Boolean) (ElapsedSeconds :type "Float (double-precision)") (TriggeredSeconds :type "Float (double-precision)") (InputAction :type "InputAction Object Reference" :default "/Game/ThirdPerson/Input/Actions/IA_Interact.IA_Interact"))
  (:`Started`
    (set `self.HidingCameraChange` true)
    (`/Engine/EditorBlueprintResources/StandardMacros.Gate` true :!label _label
      (:`Exit`
        (`self.ToggleHide`)
        (`KismetSystemLibrary.Delay` 0.2)
        (`self.SetActorHiddenInGame` false)
        (`self.EnableInput` (`GameplayStatics.GetPlayerController` 0) :!label _label_2)
        (goto _label :!via `Open`))))
  (:`Canceled`
    (set `self.HidingCameraChange` false :!label _label_3))
  (:`Completed`
    (goto _label_3)))

(event `self.Detection.OnComponentBeginOverlap`
  (params (OverlappedComponent :type "PrimitiveComponent Object Reference") (OtherActor :type "Actor Object Reference") (OtherComp :type "PrimitiveComponent Object Reference") (OtherBodyIndex :type Integer) (bFromSweep :type Boolean) (SweepResult :type "HitResult Structure (by ref)"))
  (if (== OtherActor (`self.RefThirdPersonCharacter`))
    (goto _label_2)))

(event `self.ReceiveTick`
  (params (DeltaSeconds :type "Float (single-precision)")))

(event `self.Detection.OnComponentEndOverlap`
  (params (OverlappedComponent :type "PrimitiveComponent Object Reference") (OtherActor :type "Actor Object Reference") (OtherComp :type "PrimitiveComponent Object Reference") (OtherBodyIndex :type Integer))
  (if (== OtherActor (`self.RefThirdPersonCharacter`))
    (`self.DisableInput` (`GameplayStatics.GetPlayerController` 0))
    (goto _label :!via `Close`)))

(fn `ToggleHide`
  (bind _refthirdpersoncharacter (`self.RefThirdPersonCharacter`))
  (`FMODBlueprintStatics.PlayEventAtLocation` (`self.FmodEvent1`) (`KismetMathLibrary.Conv_VectorToTransform` (`SceneComponent.GetSocketLocation` (`Character.Mesh` (`GameplayStatics.GetPlayerCharacter` 0)) "ankle_fwd_r")))
  (if (`self.IsHiding`)
    (set `self.IsHiding` false)
    (`self.HidingVignette`)
    (`self.SetActorEnableCollision` _refthirdpersoncharacter true)
    (`PlayerController.SetViewTargetWithBlend` (`GameplayStatics.GetPlayerController` 0) (`self.RefThirdPersonCharacter`) 0.6 "VTBlend_Linear" 0.0 false)
    (else
      (set `self.IsHiding` true)
      (`self.HidingVignette`)
      (`self.SetActorHiddenInGame` _refthirdpersoncharacter true)
      (`self.SetActorEnableCollision` _refthirdpersoncharacter false)
      ;[1 0 0] Causing Vignette Problems
      (`PlayerController.SetViewTargetWithBlend` (`GameplayStatics.GetPlayerController` 0) self 0.6 "VTBlend_Linear" 0.0 false))))

(fn `UserConstructionScript`
  (`parent.UserConstructionScript`))