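; Gate key pickup that an actor can interact with to add an item to an inventory.
; The construction script sets the mesh from the item data asset, and OnInteracted adds that asset to the interacting actor's inventory, destroying the pickup on success.
; A separate Interact event adds the gate key once through an inventory component and refreshes the pause-menu grid.
; GetInventory is an empty stub, and the pause-menu cast is unconnected.
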(event `self.ReceiveBeginPlay`)

(event `self.ReceiveTick`
  (params (DeltaSeconds :type "Float (single-precision)")))

(event `/Game/Interfaces/BPI_Interactable.Interact`
  (if (`self.CanInteract`)
    (set `self.CanInteract` false)
    (`/Game/Blueprints/BP_InventoryComponent.AddItem` (`self.BP_InventoryComponent1`) "/Game/Blueprints/Item_GateKey.Item_GateKey")
    (`/Game/Blueprints/UI_Pause_InventoryGrid.UpdateGrid` (`/Game/Blueprints/UI_Pause_Menu.UI_Pause_InventoryGrid` (`self.Inventory UI`)))))

(fn `GetInventory`
  (returns (Inventory :type "/Game/Blueprints/BP_InventoryComponent Object Reference"))
  (return null))

(fn `OnInteracted`
  (params (InteractingActor :type "Actor Object Reference"))
  (returns (InteractionFinished :type Boolean))
  (bind _inventory (message `/Game/Blueprints/BPI_Inventory_Interaction.GetInventory` InteractingActor))
  (`/Engine/EditorBlueprintResources/StandardMacros.IsValid` _inventory
    (:`Is Valid`
      (bind _hasfoundslot1 (`/Game/Blueprints/BP_InventoryComponent.AddItem` _inventory (`self.ItemDataAsset`)))
      (if _hasfoundslot1
        (`self.K2_DestroyActor`))
      (return _hasfoundslot1))))

(fn `UserConstructionScript`
  (bind _itemdataasset (`self.ItemDataAsset`))
  (`/Engine/EditorBlueprintResources/StandardMacros.IsValid` _itemdataasset
    (:`Is Valid`
      (`StaticMeshComponent.SetStaticMesh` (`self.StaticMesh`) (`/Game/Blueprints/BP_InventoryItem.model` _itemdataasset))
      (`parent.UserConstructionScript`))))