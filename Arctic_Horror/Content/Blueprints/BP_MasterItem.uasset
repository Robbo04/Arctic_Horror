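; Base item Blueprint that shows an animated interaction prompt when the player is nearby and interaction is allowed.
; Detection overlap creates UI_Interact in the OpenWidget component, plays its PopUp, then reverses and removes it on exit.
; CanRecieveTrace shows or hides the existing prompt through ShowWidget and HideWidget, keeping HintVisible and CanPressF in sync.
; BeginPlay also caches a BP_Enemy reference, unused in these graphs.
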(event `self.ReceiveBeginPlay`
  (bind _returnvalue (`GameplayStatics.GetActorOfClass` "/Game/Enemies/BP_Enemy.BP_Enemy_C"))
  (set `self.EnemyBP` _returnvalue))

(event `self.Detection.OnComponentBeginOverlap`
  (params (OverlappedComponent :type "PrimitiveComponent Object Reference") (OtherActor :type "Actor Object Reference") (OtherComp :type "PrimitiveComponent Object Reference") (OtherBodyIndex :type Integer) (bFromSweep :type Boolean) (SweepResult :type "HitResult Structure (by ref)"))
  (bind _openwidget (`self.OpenWidget`))
  (if (== OtherActor (`GameplayStatics.GetPlayerCharacter` 0))
    (if (not (`self.IsUIActive`))
      (set `self.IsUIActive` true)
      (if (`self.CanInteract`)
        (bind _returnvalue (`|CreateWidget` "/Game/Interfaces/UI_Interact.UI_Interact_C"))
        (bind _output_get (set `self.InteractionWidget` _returnvalue))
        (`WidgetComponent.SetWidget` _openwidget _output_get)
        (`SceneComponent.SetVisibility` _openwidget true false)
        (bind _interactionwidget (`self.InteractionWidget`)
          (:`then`
            (if (not (`self.HintVisible`))
              (`UserWidget.PlayAnimation` _interactionwidget (`/Game/Interfaces/UI_Interact.PopUp` _interactionwidget) 0.0 1 "Forward" 1.0 false)
              (set `self.HintVisible` true)
              (set `self.CanPressF` true)
              (`KismetSystemLibrary.Delay` 0.15)))
          (:`else`))))))

(event `self.Detection.OnComponentEndOverlap`
  (params (OverlappedComponent :type "PrimitiveComponent Object Reference") (OtherActor :type "Actor Object Reference") (OtherComp :type "PrimitiveComponent Object Reference") (OtherBodyIndex :type Integer))
  (if (== OtherActor (`GameplayStatics.GetPlayerCharacter` 0))
    (set `self.IsUIActive` false)
    (if (`self.CanInteract`)
      (bind _interactionwidget (`self.InteractionWidget`)
        (:`then`
          (if (`self.HintVisible`)
            (`UserWidget.PlayAnimation` _interactionwidget (`/Game/Interfaces/UI_Interact.PopUp` _interactionwidget) 0.0 1 "Reverse" 1.0 false)
            (set `self.HintVisible` false)
            (set `self.CanPressF` false))
          (`KismetSystemLibrary.Delay` 0.1)
          (`Widget.RemoveFromParent` (`self.InteractionWidget`))
          (set `self.InteractionWidget` null)
          (`SceneComponent.SetVisibility` (`self.OpenWidget`) false false))
        (:`else`)))))

(event `/Game/Interfaces/BPI_Interactable.Can Recieve Trace`
  (params (`Can Insert` :type Boolean))
  (if (`self.CanInteract`)
    (if `Can Insert`
      (`self.Show Widget`)
      (else
        (`self.Hide Widget`)))))

(fn `Hide Widget`
  (bind _interactionwidget (`self.InteractionWidget`)
    (:`then`
      (if (`self.HintVisible`)
        (`UserWidget.PlayAnimation` _interactionwidget (`/Game/Interfaces/UI_Interact.PopUp` _interactionwidget) 0.0 1 "Reverse" 1.5 false)
        (set `self.HintVisible` false)
        (set `self.CanPressF` false)))
    (:`else`)))

(fn `Show Widget`
  (bind _interactionwidget (`self.InteractionWidget`)
    (:`then`
      (if (not (`self.HintVisible`))
        (`UserWidget.PlayAnimation` _interactionwidget (`/Game/Interfaces/UI_Interact.PopUp` _interactionwidget) 0.0 1 "Forward" 1.5 false)
        (set `self.HintVisible` true)
        (set `self.CanPressF` true)))
    (:`else`)))

(fn `UserConstructionScript`)