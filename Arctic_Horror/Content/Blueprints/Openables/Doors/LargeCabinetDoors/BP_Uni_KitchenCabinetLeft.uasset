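; Kitchen cabinet left door Blueprint that the player toggles open and closed through an Interact event, gated by CanPressF and CanInteract.
; A timeline lerps the mesh yaw 90 degrees from the rotation saved at BeginPlay, playing forward to open and reversing to close.
; Opening also plays an FMOD event with an OpenType parameter.
; A short delay triggered from the timeline update re-enables interaction.
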(event `self.ReceiveBeginPlay`
  (set `self.StartingRotation` (`SceneComponent.RelativeRotation` (`self.StaticMesh`))))

(event `self.Interact`
  (bind (_startingrotation_roll _startingrotation_pitch _startingrotation_yaw) (`KismetMathLibrary.BreakRotator` (`self.StartingRotation`)))
  (if (`self.CanPressF`)
    (if (`self.CanInteract`)
      (set `self.CanInteract` false)
      (if (`self.DoorOpened`)
        (set `self.DoorOpened` false)
        (bind (_direction _alpha) (`Timeline|Timeline` :!via `Reverse` :!label _label)
          (:`Update`
            (`SceneComponent.K2_SetRelativeRotation` (`self.StaticMesh`) (`KismetMathLibrary.MakeRotator` _startingrotation_roll _startingrotation_pitch (`KismetMathLibrary.Lerp` _startingrotation_yaw (+ _startingrotation_yaw 90.0) _alpha)) false false)
            (`KismetSystemLibrary.Delay` 0.2)
            (set `self.CanInteract` true)))
        (else
          (set `self.DoorOpened` true)
          (bind _returnvalue (`FMODBlueprintStatics.PlayEventAtLocation` (`self.FmodEvent`) (`KismetMathLibrary.Conv_VectorToTransform` (`SceneComponent.K2_GetComponentLocation` (`self.StaticMesh`)))))
          (`FMODBlueprintStatics.EventInstanceSetParameter` _returnvalue "OpenType")
          (goto _label :!via `PlayFromStart`))))))

(fn `UserConstructionScript`
  (`parent.UserConstructionScript`))