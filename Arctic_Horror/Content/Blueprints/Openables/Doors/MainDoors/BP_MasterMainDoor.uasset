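; Master main door that the player pushes open by walking or crouching into it, or slams by sprinting into it.
; Overlap boxes trigger timelines that rotate the mesh yaw, with swing side set by dot product or slam box.
; Interact checks the inventory for a key, unlocking or playing a locked rattle, but its open/close state cycle is disconnected.
; Leaving the detection box swings the door shut after a delay.
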(event `self.DoorHitDetection.OnComponentBeginOverlap`
  (params (OverlappedComponent :type "PrimitiveComponent Object Reference") (OtherActor :type "Actor Object Reference") (OtherComp :type "PrimitiveComponent Object Reference") (OtherBodyIndex :type Integer) (bFromSweep :type Boolean) (SweepResult :type "HitResult Structure (by ref)"))
  (bind _thirdpersonref (`self.ThirdPersonRef`))
  (bind _staticmesh (`self.StaticMesh`))
  (bind _staticmesh_2 (`self.StaticMesh`))
  (bind (_relativerotation_roll _relativerotation_pitch _relativerotation_yaw) (`KismetMathLibrary.BreakRotator` (`SceneComponent.RelativeRotation` _staticmesh)))
  (bind (_relativerotation_roll_2 _relativerotation_pitch_2 _relativerotation_yaw_2) (`KismetMathLibrary.BreakRotator` (`SceneComponent.RelativeRotation` _staticmesh_2)))
  (if (== OtherActor _thirdpersonref)
    (`self.Is Interacting With Door` (`self.ThirdPersonRef`))
    (switch `/Game/Blueprints/E_MovementStates` (`/Game/ThirdPerson/Blueprints/BP_ThirdPersonCharacter.E_MovementState` _thirdpersonref)
      (:`NewEnumerator0`
        (bind (_direction _dooranimation) (`Timeline|FreeCrouchMovingDoorAnim` :!label _label)
          (:`Update`
            (`SceneComponent.K2_SetRelativeRotation` _staticmesh (`KismetMathLibrary.MakeRotator` 0.0 0.0 (* (`KismetMathLibrary.Lerp` 0.0 (`self.B`) _dooranimation) (`self.DoorOpenSide`))) false false))
          (:`Finished`
            (set `self.CurrentDoorRotation` _relativerotation_yaw))))
      (:`NewEnumerator1`
        (bind (_direction_2 _dooranimation_2) (`Timeline|FreeWalkMovingDoorAnim` :!label _label_2)
          (:`Update`
            (`SceneComponent.K2_SetRelativeRotation` _staticmesh_2 (`KismetMathLibrary.MakeRotator` 0.0 0.0 (* (`KismetMathLibrary.Lerp` 0.0 (`self.B`) _dooranimation_2) (`self.DoorOpenSide`))) false false))
          (:`Finished`
            (set `self.CurrentDoorRotation` _relativerotation_yaw_2)))))))

(event `StopDoorMovement`
  (`|ExecutionSequence`
    (:`then_0`
      (goto _label :!via `Stop`))
    (:`then_1`
      (goto _label_2 :!via `Stop`))))

(event `/Game/Interfaces/BPI_Interactable.Interact`
  ;[0 0 0] Door Interact
  ;;[0 0 0] Boolean Checks
  (if (`self.CanPressF`)
    (if (`self.CanInteract`)
      (set `self.CanInteract` false)
      (if (`self.isDoorLocked?`)
        ;;[0 0 0] Locked Door Functionality
        (bind _returnvalue (`self.CheckKeyItem`))
        (if _returnvalue
          (set `self.isDoorLocked?` false)
          ;;[0 0 0] Check for which side is being interacted
          (`self.Is Interacting With Door` (`self.ThirdPersonRef`) :!label _label_3)
          (else
            (bind (_direction _newtrack_0) (`Timeline|DoorLockedAnim` :!via `PlayFromStart`)
              (:`Update`
                (`SceneComponent.K2_SetRelativeRotation` (`self.StaticMesh`) (`KismetMathLibrary.MakeRotator` 0.0 0.0 (* _newtrack_0 (`self.DoorOpenSide`))) false false))
              (:`Finished`
                (`KismetSystemLibrary.PrintString` "Is locked")
                (set `self.CanInteract` true)))))
        (else
          (goto _label_3))))))

(event `ResetDoorMovement`
  (`|ExecutionSequence`
    (:`then_0`
      (goto _label :!via `SetNewTime`))
    (:`then_1`
      (goto _label_2 :!via `SetNewTime`))))

(event `self.ReceiveBeginPlay`
  ;[0 0 0] Set Third Person Reference
  (bind _returnvalue (`GameplayStatics.GetActorOfClass` "/Game/ThirdPerson/Blueprints/BP_ThirdPersonCharacter.BP_ThirdPersonCharacter_C"))
  (set `self.ThirdPersonRef` _returnvalue))

(event `self.DoorHitDetection.OnComponentEndOverlap`
  (params (OverlappedComponent :type "PrimitiveComponent Object Reference") (OtherActor :type "Actor Object Reference") (OtherComp :type "PrimitiveComponent Object Reference") (OtherBodyIndex :type Integer))
  (if (== OtherActor (`self.ThirdPersonRef`))
    _))

(event `self.Detection.OnComponentEndOverlap`
  (params (OverlappedComponent :type "PrimitiveComponent Object Reference") (OtherActor :type "Actor Object Reference") (OtherComp :type "PrimitiveComponent Object Reference") (OtherBodyIndex :type Integer))
  ;[0 0 0] Checks if player has left detection box
  (if (== OtherActor (`self.ThirdPersonRef`))
    ;[1 0 0] TBC
    (`KismetSystemLibrary.Delay` 3.0)
    (bind (_direction _newtrack_0) (`Timeline|Reset Door Animation`)
      (:`Update`
        (`SceneComponent.K2_SetRelativeRotation` (`self.StaticMesh`) (`KismetMathLibrary.MakeRotator` 0.0 0.0 (`KismetMathLibrary.Lerp` (`self.CurrentDoorRotation`) 0.0 _newtrack_0)) false false))
      (:`Finished`
        (`self.ResetDoorMovement`)))))

(event `CustomEvent_0`
  ;[0 0 0] Switches Door Enum State to next open type (open, partially open, closed)
  (switch `/Game/Blueprints/E_DoorStates` (`self.EDoorStates`)
    (:`NewEnumerator0`
      (set `self.EDoorStates` "NewEnumerator1"))
    (:`NewEnumerator1`
      (set `self.EDoorStates` "NewEnumerator2"))
    (:`NewEnumerator2`
      (set `self.EDoorStates` "NewEnumerator0")))
  (set `self.CanInteract` true))

(event `Is Interacting With Door`
  (params (Target :type "Actor Object Reference"))
  ;[0 0 0] Detect Which Side the player is on when interacting with the door
  (if (> (`KismetMathLibrary.Dot_VectorVector` (`self.GetActorForwardVector` Target) (`SceneComponent.GetForwardVector` (`self.OriginReferencePoint`))) 0.0)
    (set `self.DoorOpenSide` -1.0)
    (else
      (set `self.DoorOpenSide` 1.0))))

(event `self.Front.OnComponentBeginOverlap`
  (params (OverlappedComponent :type "PrimitiveComponent Object Reference") (OtherActor :type "Actor Object Reference") (OtherComp :type "PrimitiveComponent Object Reference") (OtherBodyIndex :type Integer) (bFromSweep :type Boolean) (SweepResult :type "HitResult Structure (by ref)"))
  (bind (_relativerotation_roll _relativerotation_pitch _relativerotation_yaw) (`KismetMathLibrary.BreakRotator` (`SceneComponent.RelativeRotation` (`self.StaticMesh`))))
  ;[0 0 0] Door Slam
  ;;[0 0 0] Detects that player is interacting with door
  (if (== OtherActor (`GameplayStatics.GetPlayerCharacter` 0))
    ;;[0 0 0] Is Player Running at Door?
    (if (`/Game/ThirdPerson/Blueprints/BP_ThirdPersonCharacter.IsSprinting` (`self.ThirdPersonRef`))
      ;;[0 0 0] Sets Side Player is Running Into
      (set `self.DoorOpenSide` -1.0)
      ;;[0 0 0] Checks that door is closed
      (if (== _relativerotation_yaw 0.0)
        ;;[0 0 0] Slam Anims when Door is Closed
        (bind (_direction _slamfront) (`Timeline|DoorSlamFrontAnim` :!via `PlayFromStart`)
          (:`Update`
            (`SceneComponent.K2_SetRelativeRotation` (`self.StaticMesh`) (`KismetMathLibrary.MakeRotator` 0.0 0.0 (* _slamfront (`self.DoorOpenSide`))) false false))
          (:`Finished`
            (set `self.Door Slammed` true)))
        (else
          ;;[0 0 0] Partially Open
          (if (== (`self.EDoorStates`) 1) :!label _label_4
            ;;[0 0 0] Check Which side running into
            (if (== (`self.DoorOpenSide`) -1.0)
              ;;[0 0 0] Slam Anims when Door is Partially Open
              (bind (_direction_2 _slamfront_2) (`Timeline|DoorSlamFrontPOAnim` :!via `PlayFromStart`)
                (:`Update`
                  (`SceneComponent.K2_SetRelativeRotation` (`self.StaticMesh`) (`KismetMathLibrary.MakeRotator` 0.0 0.0 (* _slamfront_2 (`self.DoorOpenSide`))) false false))
                (:`Finished`
                  (set `self.Door Slammed` true)))
              (elif (== (`self.DoorOpenSide`) 1.0)
                (bind (_direction_3 _slam_rear) (`Timeline|DoorSlamRearPOAnim` :!via `PlayFromStart`)
                  (:`Update`
                    (`SceneComponent.K2_SetRelativeRotation` (`self.StaticMesh`) (`KismetMathLibrary.MakeRotator` 0.0 0.0 (* _slam_rear (`self.DoorOpenSide`))) false false))
                  (:`Finished`
                    (set `self.Door Slammed` true)))))))))))

(event `self.Rear.OnComponentBeginOverlap`
  (params (OverlappedComponent :type "PrimitiveComponent Object Reference") (OtherActor :type "Actor Object Reference") (OtherComp :type "PrimitiveComponent Object Reference") (OtherBodyIndex :type Integer) (bFromSweep :type Boolean) (SweepResult :type "HitResult Structure (by ref)"))
  (bind (_relativerotation_roll _relativerotation_pitch _relativerotation_yaw) (`KismetMathLibrary.BreakRotator` (`SceneComponent.RelativeRotation` (`self.StaticMesh`))))
  ;[0 0 0] Door Slam
  ;;[0 0 0] Detects that player is interacting with door
  (if (== OtherActor (`GameplayStatics.GetPlayerCharacter` 0))
    ;;[0 0 0] Is Player Running at Door?
    (if (`/Game/ThirdPerson/Blueprints/BP_ThirdPersonCharacter.IsSprinting` (`self.ThirdPersonRef`))
      ;;[0 0 0] Sets Side Player is Running Into
      (set `self.DoorOpenSide` 1.0)
      ;;[0 0 0] Checks that door is closed
      (if (== _relativerotation_yaw 0.0)
        ;;[0 0 0] Slam Anims when Door is Closed
        (bind (_direction _slam_rear) (`Timeline|DoorSlamRearAnim`)
          (:`Update`
            (`SceneComponent.K2_SetRelativeRotation` (`self.StaticMesh`) (`KismetMathLibrary.MakeRotator` 0.0 0.0 (* _slam_rear (`self.DoorOpenSide`))) false false))
          (:`Finished`
            (set `self.Door Slammed` true)))
        (else
          (goto _label_4))))))

(fn `CheckKeyItem`
  (returns (ReturnValue :type Boolean))
  (bind _inventory (message `/Game/Blueprints/BPI_Inventory_Interaction.GetInventory` (`GameplayStatics.GetPlayerCharacter` 0)))
  (bind _hasgatekey (`/Game/Blueprints/BP_InventoryComponent.CheckForItem` _inventory))
  (bind _output_get (set `self.hasCorrectKey?` _hasgatekey))
  (if _output_get
    (return _output_get)))

(fn `IsInteractingWithDoor`
  (params (self2 :type "SceneComponent Object Reference"))
  (if (> (`KismetMathLibrary.Dot_VectorVector` (`self.GetActorForwardVector`) (`SceneComponent.GetForwardVector` self2)) 0.0)
    (set `self.DoorOpenSide` -1.0)
    (else
      (set `self.DoorOpenSide` 1.0)))
  (return))

(fn `UserConstructionScript`
  (`parent.UserConstructionScript`))