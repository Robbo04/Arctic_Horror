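; BP_Uni_KitchenSmallDraw is an interactable small kitchen drawer that slides open and closed.
; Interact, gated by CanPressF and CanInteract, toggles CabinetOpened and plays the SmallDrawAnimation timeline from start to open or in reverse to close.
; Each update adds the opening or closing track value to the mesh's relative X location, so movement accumulates per tick.
; Interaction re-enables shortly after the timeline finishes.
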(event `/Game/Interfaces/BPI_Interactable.Interact`
  (bind _staticmesh (`self.StaticMesh`))
  (if (`self.CanPressF`)
    (if (`self.CanInteract`)
      (set `self.CanInteract` false)
      (if (`self.CabinetOpened`)
        (set `self.CabinetOpened` false)
        (bind (_direction _openingtrack _closingtrack) (`Timeline|SmallDrawAnimation` :!via `Reverse` :!label _label)
          (:`Update`
            (if (`self.CabinetOpened`)
              (`SceneComponent.K2_AddRelativeLocation` _staticmesh (`KismetMathLibrary.MakeVector` _openingtrack) false false)
              (else
                (`SceneComponent.K2_AddRelativeLocation` _staticmesh (`KismetMathLibrary.MakeVector` _closingtrack) false false))))
          (:`Finished`
            (`KismetSystemLibrary.Delay` 0.2)
            (set `self.CanInteract` true)))
        (else
          (set `self.CabinetOpened` true)
          (goto _label :!via `PlayFromStart`))))))

(fn `UserConstructionScript`
  (`parent.UserConstructionScript`))