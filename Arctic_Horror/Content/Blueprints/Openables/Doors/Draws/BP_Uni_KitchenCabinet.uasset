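; Interactable kitchen cabinet in the Draws folder that slides its static mesh open and closed along relative X.
; Interact checks CanPressF and a CanInteract lock, toggles CabinetOpened, and plays an FMOD open or close event at the mesh with an OpenType parameter.
; A timeline plays forward or in reverse, adding per-update offsets from separate opening and closing tracks, then releases the lock after a short delay.
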(event `self.ReceiveTick`
  (params (DeltaSeconds :type "Float (single-precision)")))

(event `/Game/Interfaces/BPI_Interactable.Interact`
  (bind _staticmesh (`self.StaticMesh`))
  (bind _returnvalue (`KismetMathLibrary.Conv_VectorToTransform` (`SceneComponent.K2_GetComponentLocation` (`self.StaticMesh`))))
  (if (`self.CanPressF`)
    (if (`self.CanInteract`)
      (set `self.CanInteract` false)
      (if (`self.CabinetOpened`)
        (set `self.CabinetOpened` false)
        (bind _returnvalue_2 (`FMODBlueprintStatics.PlayEventAtLocation` (`self.FmodEvent2`) _returnvalue))
        (`FMODBlueprintStatics.EventInstanceSetParameter` _returnvalue_2 "OpenType" 2.0)
        (bind (_direction _openingtrack _closingtrack) (`Timeline|Timeline_0` :!via `Reverse` :!label _label)
          (:`Update`
            (if (`self.CabinetOpened`)
              (`SceneComponent.K2_AddRelativeLocation` _staticmesh (`KismetMathLibrary.MakeVector` _openingtrack) false false)
              (else
                (`SceneComponent.K2_AddRelativeLocation` _staticmesh (`KismetMathLibrary.MakeVector` _closingtrack) false false))))
          (:`Finished`
            (`KismetSystemLibrary.Delay` 0.2)
            (set `self.CanInteract` true)))
        (else
          (set `self.CabinetOpened` true)
          (bind _returnvalue_3 (`FMODBlueprintStatics.PlayEventAtLocation` (`self.FmodEvent1`) _returnvalue))
          (`FMODBlueprintStatics.EventInstanceSetParameter` _returnvalue_3 "OpenType" 2.0)
          (goto _label :!via `PlayFromStart`))))))

(fn `UserConstructionScript`
  (`parent.UserConstructionScript`))