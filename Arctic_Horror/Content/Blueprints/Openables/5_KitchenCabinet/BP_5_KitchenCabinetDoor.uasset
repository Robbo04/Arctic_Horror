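; Kitchen cabinet door actor that swings open or closed on the Interact event.
; Interact requires CanPressF and CanInteract, then flips DoorOpened and plays the Timeline forward from start or in reverse.
; The Timeline drives the static mesh's relative yaw.
; CanInteract is cleared on use and set false again after a short post-finish delay, so nothing in this graph re-enables interaction.
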(event `/Game/Interfaces/BPI_Interactable.Interact`
  (if (`self.CanPressF`)
    (if (`self.CanInteract`)
      (set `self.CanInteract` false)
      (if (`self.DoorOpened`)
        (set `self.DoorOpened` false)
        (bind (_direction _animationtrack) (`Timeline|Timeline` :!via `Reverse` :!label _label)
          (:`Update`
            (`SceneComponent.K2_SetRelativeRotation` (`self.StaticMesh`) (`KismetMathLibrary.MakeRotator` 0.0 0.0 _animationtrack) false false))
          (:`Finished`
            (`KismetSystemLibrary.Delay` 0.2)
            (set `self.CanInteract` false)))
        (else
          (set `self.DoorOpened` true)
          (goto _label :!via `PlayFromStart`))))))

(fn `UserConstructionScript`
  (`parent.UserConstructionScript`))