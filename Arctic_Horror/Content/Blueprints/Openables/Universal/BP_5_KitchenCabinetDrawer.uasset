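; BP_5_KitchenCabinetDrawer is an openable kitchen cabinet drawer that slides open or closed on interaction.
; Interact checks CanPressF and CanInteract, then toggles CabinetOpened and plays a timeline forward from the start or in reverse.
; Each timeline update adds the track value to the mesh's relative X as a delta rather than setting a position.
; Interaction stays locked until a short delay after the timeline finishes.
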(event `/Game/Interfaces/BPI_Interactable.Interact`
  (if (`self.CanPressF`)
    (if (`self.CanInteract`)
      (set `self.CanInteract` false)
      (if (`self.CabinetOpened`)
        (set `self.CabinetOpened` false)
        (bind (_direction _animationtrack) (`Timeline|Timeline` :!via `Reverse` :!label _label)
          (:`Update`
            (`SceneComponent.K2_AddRelativeLocation` (`self.StaticMesh`) (`KismetMathLibrary.MakeVector` _animationtrack) false false))
          (:`Finished`
            (`KismetSystemLibrary.Delay` 0.2)
            (set `self.CanInteract` true)))
        (else
          (set `self.CabinetOpened` true)
          (goto _label :!via `PlayFromStart`))))))

(fn `UserConstructionScript`
  (`parent.UserConstructionScript`))