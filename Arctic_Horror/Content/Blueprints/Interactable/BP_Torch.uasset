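; Hand-crank torch with a battery that drains while the spotlight is on, switching off when empty and needing a minimum charge to turn on.
; While off, Tick recharges it slowly from held winding or faster from repeated taps, which a looping timer resets.
; Timelines animate switch and winder, with FMOD sounds for toggling and held winding.
; Flicker alternates two intensity timelines on the spotlight.
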(event `self.ReceiveTick`
  (params (DeltaSeconds :type "Float (single-precision)"))
  (set `self.Delta Seconds` DeltaSeconds)
  (`|ExecutionSequence`
    (:`then_0`
      ;[0 0 0] Switch Timeline
      (if (`self.IsTurnedOn`)
        (bind (_direction _switch_float) (`Timeline|SwitchAnimGraph` :!label _label)
          (:`Update`
            (`SceneComponent.K2_SetRelativeRotation` (`self.Switch`) (`KismetMathLibrary.MakeRotator` 0.0 _switch_float) false false)))
        (elif (not (`self.IsTurnedOn`))
          (goto _label :!via `Reverse`))))
    (:`then_1`
      ;[0 0 0] Fast Carge Timeline
      (if (`self.FastCharge`)
        (bind (_direction_2 _windfloat) (`Timeline|WinderFastAnimGraph` :!label _label_2)
          (:`Update`
            (if (not (>= (`self.BatteryLife`) 100.0))
              (`SceneComponent.K2_SetRelativeRotation` (`self.Winder`) (`KismetMathLibrary.MakeRotator` 0.0 _windfloat) false false))))
        (else
          (goto _label_2 :!via `Stop`))))
    (:`then_2`
      ;[0 0 0] Slow Charge Timeline
      (if (`self.ChargingActive`)
        (bind (_direction_3 _wind_float) (`Timeline|WinderSlowAnimGraph`)
          (:`Update`
            (if (`self.ChargingActive`)
              (if (not (>= (`self.BatteryLife`) 100.0))
                (`SceneComponent.K2_SetRelativeRotation` (`self.Winder`) (`KismetMathLibrary.MakeRotator` 0.0 _wind_float) false false)))))))
    (:`then_3`
      (if (`self.IsTurnedOn`)
        ;[0 0 0 1 30] DRAIN BATTERY
        (if (> (`self.BatteryLife`) 0.0)
          (bind _output_get (set `self.BatteryLife` (- (`self.BatteryLife`) (* (`self.Delta Seconds`) 3.0))))
          (if (not (> _output_get 100.0))
            (`KismetSystemLibrary.PrintString` (`KismetStringLibrary.Conv_DoubleToString` (`self.BatteryLife`)) true true (struct :`G` 0.66 :`B` 1.0 :`A` 1.0) 0.1 :!label _label_3))
          (else
            (`self.SwitchOn/Off`)))
        (else
          ;[0 0 0 1 30] RECHARGE
          (if (`self.FastCharge`)
            (set `self.BatteryLife` (+ (* (`self.Delta Seconds`) 10.0) (`self.BatteryLife`)))
            ;[0 0 0] STOP WHEN FULL
            (if (>= (`self.BatteryLife`) 100.0) :!label _label_4
              (set `self.BatteryLife` 100.0)
              (goto _label_3)
              (else
                (goto _label_3)))
            (elif (`self.ChargingActive`)
              (set `self.BatteryLife` (+ (* (`self.Delta Seconds`) 5.0) (`self.BatteryLife`)))
              (goto _label_4))))))))

(event `TapCharge`
  (bind _fastchargecounter (`self.FastChargeCounter`))
  ;[0 0 0 1 30] Tapping to charge
  (`KismetSystemLibrary.K2_SetTimerDelegate` (delegate `StopTapCharge`) 0.6 true)
  (bind _result (`/Engine/EditorBlueprintResources/StandardMacros.IncrementInt` _fastchargecounter)
    (:`  `
      (if (> _fastchargecounter 1)
        (set `self.FastCharge` true))
      (`KismetSystemLibrary.PrintString` (`KismetStringLibrary.Conv_IntToString` _result)))))

(event `StopTapCharge`
  ;[0 0 0 1 30] Tapping to charge
  (if (`self.FastCharge`)
    (set `self.FastCharge` false)
    (`KismetSystemLibrary.PrintString` "Stopped Quick Charge" true true (struct :`R` 1.0 :`A` 1.0)))
  (set `self.FastChargeCounter` 0))

(event `ChargeActivate`
  (params (ShouldActivate :type Boolean))
  (bind _fmodcharge (`self.FMODCharge`))
  ;[0 0 0 1 30] Holding charge function
  (bind _output_get (set `self.ChargingActive` ShouldActivate))
  (if _output_get
    (`FMODAudioComponent.SetParameter` (`self.FMODCharge`) "WindingState" 1.0)
    (`FMODAudioComponent.Play` (`self.FMODCharge`))
    (else
      (`FMODAudioComponent.SetParameter` _fmodcharge "WindingState" 0.0)
      (`FMODAudioComponent.Stop` _fmodcharge))))

(event `Flicker`
  (bind _spotlight (`self.SpotLight`))
  (`/Engine/EditorBlueprintResources/StandardMacros.DoOnce` false :!label _label_5
    (:`Completed`
      (`/Engine/EditorBlueprintResources/StandardMacros.FlipFlop`
        (:`A`
          (bind (_direction _newtrack_0) (`Timeline|Timeline` :!via `PlayFromStart`)
            (:`Update`
              (`LightComponent.SetIntensity` _spotlight (* _newtrack_0 (`self.MaxBrightness`))))
            (:`Finished`
              (goto _label_5 :!via `Reset`))))
        (:`B`
          (bind (_direction_2 _newtrack_0_2) (`Timeline|Timeline_0` :!via `PlayFromStart`)
            (:`Update`
              (`LightComponent.SetIntensity` _spotlight (* _newtrack_0_2 (`self.MaxBrightness`))))
            (:`Finished`
              (goto _label_5 :!via `Reset`))))))))

(fn `SwitchOn/Off`
  (bind _spotlight (`self.SpotLight`))
  (`FMODAudioComponent.Play` (`self.FMODTorchon/off`))
  (if (not (`self.IsTurnedOn`))
    (if (and (not (`self.IsTurnedOn`)) (>= (`self.BatteryLife`) 10.0))
      (`SceneComponent.SetVisibility` _spotlight true false)
      (set `self.IsTurnedOn` true))
    (else
      (`SceneComponent.SetVisibility` _spotlight false false)
      (set `self.IsTurnedOn` false))))

(fn `UserConstructionScript`)