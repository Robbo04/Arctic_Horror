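; BP_HidingPlace is an interactable hiding spot that flags the player as hidden while inside its box volume.
; Player overlap begin and end write the PlayerIsHiding blackboard key true and false on the single BP_Enemy returned by GetActorOfClass.
; It also sets IsHiding on the character cached at BeginPlay, but both events set it true, so leaving never clears that flag.
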(event `self.ReceiveBeginPlay`
  (bind _returnvalue (`GameplayStatics.GetActorOfClass` "/Game/ThirdPerson/Blueprints/BP_ThirdPersonCharacter.BP_ThirdPersonCharacter_C"))
  (set `self.TPC` _returnvalue))

(event `self.Box.OnComponentBeginOverlap`
  (params (OverlappedComponent :type "PrimitiveComponent Object Reference") (OtherActor :type "Actor Object Reference") (OtherComp :type "PrimitiveComponent Object Reference") (OtherBodyIndex :type Integer) (bFromSweep :type Boolean) (SweepResult :type "HitResult Structure (by ref)"))
  (if (== OtherActor (`GameplayStatics.GetPlayerCharacter` 0))
    (set `/Game/ThirdPerson/Blueprints/BP_ThirdPersonCharacter.IsHiding` true (`self.TPC`))
    (bind _returnvalue (`GameplayStatics.GetActorOfClass` "/Game/Enemies/BP_Enemy.BP_Enemy_C"))
    (`BlackboardComponent.SetValueAsBool` (`AIBlueprintHelperLibrary.GetBlackboard` _returnvalue) (`self.Player Is Hiding Key Name`) true)))

(event `self.Box.OnComponentEndOverlap`
  (params (OverlappedComponent :type "PrimitiveComponent Object Reference") (OtherActor :type "Actor Object Reference") (OtherComp :type "PrimitiveComponent Object Reference") (OtherBodyIndex :type Integer))
  (if (== OtherActor (`GameplayStatics.GetPlayerCharacter` 0))
    (set `/Game/ThirdPerson/Blueprints/BP_ThirdPersonCharacter.IsHiding` true (`self.TPC`))
    (bind _returnvalue (`GameplayStatics.GetActorOfClass` "/Game/Enemies/BP_Enemy.BP_Enemy_C"))
    (`BlackboardComponent.SetValueAsBool` (`AIBlueprintHelperLibrary.GetBlackboard` _returnvalue) (`self.Player Is Hiding Key Name`) false)))

(fn `UserConstructionScript`)