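; BP_Door is an interactable door that swings open and closed on its hinge.
; Each Interact call prints a debug "Hello" and flip-flops between playing and reversing a Timeline.
; The Timeline track scales the Hinge's relative yaw up to a quarter turn, feeding its world roll and pitch into that relative rotation.
; BeginPlay caches the hinge's starting transform, which the graph never reads.
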(event `self.ReceiveBeginPlay`
  (set `self.StartingTransform` (`SceneComponent.K2_GetComponentToWorld` (`self.Hinge`))))

(event `self.ReceiveTick`
  (params (DeltaSeconds :type "Float (single-precision)")))

(event `/Game/Interfaces/BPI_Interactable.Interact`
  (bind (_returnvalue_roll _returnvalue_pitch) (`KismetMathLibrary.BreakRotator` (`SceneComponent.K2_GetComponentRotation` (`self.Hinge`))))
  (`KismetSystemLibrary.PrintString` "Hello")
  (`/Engine/EditorBlueprintResources/StandardMacros.FlipFlop`
    (:`A`
      (bind (_direction _newtrack_0) (`Timeline|Timeline` :!label _label)
        (:`Update`
          (`SceneComponent.K2_SetRelativeRotation` (`self.Hinge`) (`KismetMathLibrary.MakeRotator` _returnvalue_roll _returnvalue_pitch (* _newtrack_0 90.0)) false false))))
    (:`B`
      (goto _label :!via `Reverse`))))

(fn `UserConstructionScript`)