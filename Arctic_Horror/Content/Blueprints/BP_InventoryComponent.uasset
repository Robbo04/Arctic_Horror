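; BP_InventoryComponent is a slot-based item inventory that fills an array to InventorySize on BeginPlay.
; AddItem seeks a same-item slot whose StackSize exceeds the item's, else fills the first empty slot, returning whether either succeeded.
; That same-item branch writes HasItem false and index+1 as StackSize, rather than incrementing the stack.
; RemoveItem finds the item's slot, then decrements its stack or clears it.
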(event `self.ReceiveBeginPlay`
  (`self.InventoryConstructor`))

(fn `AddItem`
  (params (ItemToAdd :type "/Game/Blueprints/BP_InventoryItem Object Reference"))
  (returns (HasFoundSlot1 :type Boolean))
  (locals (`Has Found Slot` :type Boolean))
  (bind _has_found_slot (`local.Has Found Slot`))
  (for (_array_element _array_index) (`self.Inventory`)
    (bind (_hasitem _stacksize _itemasset) (break `/Game/Blueprints/STO_InventorySlot` _array_element))
    (if (and _hasitem (== ItemToAdd _itemasset) (> _stacksize (`/Game/Blueprints/BP_InventoryItem.StackSize` ItemToAdd)))
      (`KismetArrayLibrary.Array_Set` (`self.Inventory`) _array_index (make `/Game/Blueprints/STO_InventorySlot` false (+ _array_index 1) ItemToAdd))
      (set `local.Has Found Slot` true)
      (break)))
  (`KismetSystemLibrary.PrintString` "Item Can Be Added To Inventory")
  (if _has_found_slot
    (return _has_found_slot)
    (else
      (for (_array_element_2 _array_index_2) (`self.Inventory`)
        (if (not (`.HasItem_1_4097ABDA47943E371E4358B28B4656E0` (break `/Game/Blueprints/STO_InventorySlot` _array_element_2)))
          (`KismetArrayLibrary.Array_Set` (`self.Inventory`) _array_index_2 (make `/Game/Blueprints/STO_InventorySlot` true 1 ItemToAdd))
          (set `local.Has Found Slot` true)
          (break)))
      (`KismetSystemLibrary.PrintString` "Has Added Item To Inventory")
      (return (`local.Has Found Slot`)))))

(fn `InventoryConstructor`
  (bind _inventory (`self.Inventory`))
  (`KismetArrayLibrary.Array_Clear` _inventory)
  (for _ (range (`self.InventorySize`))
    (`KismetArrayLibrary.Array_Add` _inventory)))

(fn `RemoveItem`
  (params (ItemToAdd :type "/Game/Blueprints/STO_InventorySlot Structure"))
  (bind _inventory (`self.Inventory`))
  (bind _output (`|GetArrayItem` _inventory (`KismetArrayLibrary.Array_Find` _inventory ItemToAdd)))
  (bind (_hasitem _stacksize _itemasset) (break `/Game/Blueprints/STO_InventorySlot` _output))
  (if (> _stacksize 1)
    (bind _result (`/Engine/EditorBlueprintResources/StandardMacros.DecrementInt` _stacksize)
      (:`  `
        (`|VariableSetRef` _output (make `/Game/Blueprints/STO_InventorySlot` true _result _itemasset))))
    (else
      (`|VariableSetRef` _output (make `/Game/Blueprints/STO_InventorySlot` false))))
  (return))