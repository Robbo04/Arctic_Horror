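; BP_SetNewSpline is a trigger volume that changes the enemy's spline route while the player is inside it.
; On BeginPlay it finds a single BP_Enemy through GetActorOfClass and caches that enemy's original SplineRoute.
; When the player character begins overlapping BoxCollision, it assigns its own Spline to the enemy's SplineRoute.
; When the player leaves the box, it restores the cached original route.
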(event `self.ReceiveBeginPlay`
  (bind _returnvalue (`GameplayStatics.GetActorOfClass` "/Game/Enemies/BP_Enemy.BP_Enemy_C"))
  (bind _output_get (set `self.Enemy` _returnvalue))
  (set `self.OGSpline` (`/Game/Enemies/BP_Enemy.SplineRoute` _output_get)))

(event `self.BoxCollision.OnComponentBeginOverlap`
  (params (OverlappedComponent :type "PrimitiveComponent Object Reference") (OtherActor :type "Actor Object Reference") (OtherComp :type "PrimitiveComponent Object Reference") (OtherBodyIndex :type Integer) (bFromSweep :type Boolean) (SweepResult :type "HitResult Structure (by ref)"))
  (if (== OtherActor (`GameplayStatics.GetPlayerCharacter` 0))
    (set `/Game/Enemies/BP_Enemy.SplineRoute` (`self.Spline`) (`self.Enemy`))))

(event `self.BoxCollision.OnComponentEndOverlap`
  (params (OverlappedComponent :type "PrimitiveComponent Object Reference") (OtherActor :type "Actor Object Reference") (OtherComp :type "PrimitiveComponent Object Reference") (OtherBodyIndex :type Integer))
  (if (== OtherActor (`GameplayStatics.GetPlayerCharacter` 0))
    (set `/Game/Enemies/BP_Enemy.SplineRoute` (`self.OGSpline`) (`self.Enemy`))))

(fn `UserConstructionScript`)