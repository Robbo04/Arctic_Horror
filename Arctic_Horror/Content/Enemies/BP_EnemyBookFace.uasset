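; Book-face enemy that screams at the player, patrols spline routes and makes melee attacks.
; Equipping its weapon snaps it toward the player and plays a scream montage; attack notifies sphere-trace forward to deal blockable damage.
; Patrol setup alternates between investigating and patrolling routes, while functions expose ranges, movement speed and damage handling through its damage component.
; Tick uses latent delays to space out breath and chain sounds.
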(event `/Game/Enemies/AI/BPI_EnemyAI.EquipWeapon`
  (`self.K2_SetActorRotation` (`KismetMathLibrary.FindLookAtRotation` (`self.K2_GetActorLocation`) (`self.K2_GetActorLocation` (`GameplayStatics.GetPlayerCharacter` 0))) true)
  (set `MovementComponent.Velocity` (0.0 0.0 0.0) (`self.CharacterMovement`))
  (`FMODAudioComponent.Play` (`self.FMODScream`))
  (`|PlayMontage` (`self.Mesh`) "/Game/Characters/BookHeadMonster/Demo/Animations/AM_ZombieScream.AM_ZombieScream" 0.8
    (:`OnCompleted`
      (`self.OnequipWeapon`)
      (set `self.IsWieldingWeapon` true))))

(event `self.ReceiveTick`
  (params (DeltaSeconds :type "Float (single-precision)"))
  (`KismetSystemLibrary.Delay` (`KismetMathLibrary.Conv_IntToDouble` (`KismetMathLibrary.RandomIntegerInRange` 10 30)))
  (`FMODAudioComponent.Play` (`self.FMODBreath`))
  (`KismetSystemLibrary.Delay` 5.0)
  (`FMODAudioComponent.Play` (`self.FMODChains`)))

(event `self.ReceiveBeginPlay`
  (`parent.ReceiveBeginPlay`))

(event `/Game/Enemies/AI/BPI_EnemyAI.Attack`
  (bind _returnvalue (`self.K2_GetActorLocation`))
  (bind _bpc_damagecomponent (`self.BPC_DamageComponent`))
  (bind _notifyname (`|PlayMontage` (`self.Mesh`) "/Game/ThirdPerson/Animations/Manny/AM_ZombieAttack.AM_ZombieAttack")
    (:`then`
      (set `/Game/DamageSystem/BPC_DamageComponent.IsInterruptable` false _bpc_damagecomponent))
    (:`OnCompleted`
      (set `/Game/DamageSystem/BPC_DamageComponent.IsInterruptable` false _bpc_damagecomponent :!label _label)
      (`self.OnAttackEnd`))
    (:`OnInterrupted`
      (goto _label))
    (:`OnNotifyBegin`
      (switch `name` _notifyname
        (:`TraceHit`
          (bind _outhit (`KismetSystemLibrary.SphereTraceSingleForObjects` _returnvalue (+ _returnvalue (* (`self.GetActorForwardVector`) 200.0)) 40.0 (`|MakeArray` "ObjectTypeQuery3" :!type "EObjectTypeQuery Enum")))
          (if true
            (bind _wasdamaged (message `/Game/DamageSystem/BPI_DamageInterface.TakeDamage` (`.HitActor` (`GameplayStatics.BreakHitResult` _outhit)) (make `/Game/DamageSystem/S_DamageInfo` 20.0 false true)))
            (if _wasdamaged
              _)))))))

(event `/Game/Enemies/AI/BPI_EnemyAI.UnequipWeapon`
  (`KismetSystemLibrary.Delay` 4.0)
  (`self.OnUnequipWeapon`)
  (set `self.IsWieldingWeapon` false))

(event `/Game/Enemies/AI/BPI_EnemyAI.SetPatrolRoute`
  (`/Engine/EditorBlueprintResources/StandardMacros.FlipFlop`
    (:`A`
      (bind _returnvalue (`GameplayStatics.GetActorOfClass` "/Game/Enemies/AI/BP_InvestigatingRoute.BP_InvestigatingRoute_C"))
      (set `self.SplineRoute` _returnvalue))
    (:`B`
      (bind _returnvalue_2 (`GameplayStatics.GetActorOfClass` "/Game/Enemies/AI/BP_PatrollingRoute.BP_PatrollingRoute_C"))
      (set `self.SplineRoute` _returnvalue_2))))

(fn `GetIdealRange`
  (returns (AttackRadius :type "Float (double-precision)") (DefendRadius :type "Float (double-precision)"))
  (return 150.0 350.0))

(fn `getPatrolRoute`
  (returns (PatrolRoute :type "/Game/Enemies/AI/BP_SplineBase Object Reference"))
  (return (`self.SplineRoute`)))

(fn `SetMovementSpeed`
  (params (SpeedEnum :type "/Game/Enemies/AI/Enums/E_MovementSpeed Enum" :default "NewEnumerator0"))
  (returns (SpeedValue :type "Float (double-precision)"))
  (bind _output_get (set `CharacterMovementComponent.MaxWalkSpeed` (select `/Game/Enemies/AI/Enums/E_MovementSpeed` SpeedEnum :`NewEnumerator1` (`self.Walking`) :`NewEnumerator2` (`self.Jogging`) :`NewEnumerator3` (`self.Sprinting`)) (`self.CharacterMovement`)))
  (return _output_get))

(fn `TakeDamage`
  (params (DamageInfo :type "/Game/DamageSystem/S_DamageInfo Structure"))
  (returns (WasDamaged :type Boolean))
  (bind _wasdamaged (`/Game/DamageSystem/BPC_DamageComponent.TakeDamage` (`self.BPC_DamageComponent`) DamageInfo))
  (return _wasdamaged))

(fn `UserConstructionScript`
  (`parent.UserConstructionScript`))