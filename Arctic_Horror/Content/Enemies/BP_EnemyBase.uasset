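; Base enemy character that delegates health, healing and damage to BPCDamageComponent and drives AI states on its AIC_Enemy_Base controller.
; Construction binds the component's death, block and damage-response events and sets starting health.
; Hits freeze the AI during a reaction montage, then resume attacking the last target; death ragdolls the mesh, stops AI logic and destroys the actor after a delay.
; Range, patrol route and movement-speed functions return empty defaults.
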(event `self.ReceiveBeginPlay`
  (bind _asaic_enemy_base (cast `/Game/Enemies/AI/AIC_Enemy_Base` (`AIBlueprintHelperLibrary.GetAIController` self)))
  (set `self.AICEnemyBase` _asaic_enemy_base))

(event `Death`
  (bind _mesh (`self.Mesh`))
  (`PrimitiveComponent.SetSimulatePhysics` _mesh true)
  (`PrimitiveComponent.SetCollisionEnabled` _mesh "QueryAndPhysics")
  (`BrainComponent.StopLogic` (`AIController.BrainComponent` (`self.AICEnemyBase`)) "")
  (`/Game/Enemies/AI/AIC_Enemy_Base.SetStateAsDead` (`self.AICEnemyBase`))
  (`ActorComponent.K2_DestroyComponent` (`self.HealthBar`))
  (`PrimitiveComponent.SetCollisionEnabled` (`self.CapsuleComponent`) "NoCollision")
  (`KismetSystemLibrary.Delay` 10.0)
  (`self.K2_DestroyActor`))

(event `Blocked`
  (`KismetSystemLibrary.PrintString` "BLOCKED"))

(event `DamageResponce`
  (params (DamageResponce :type "/Game/DamageSystem/E_DamageResponce Enum" :default "NewEnumerator0"))
  (bind _aicenemybase (`self.AICEnemyBase`))
  (`MovementComponent.StopMovementImmediately` (`self.CharacterMovement`))
  (`/Game/Enemies/AI/AIC_Enemy_Base.SetStateAsFrozen` _aicenemybase)
  (`|PlayMontage` (`self.Mesh`) (`self.HitReactionMontage`) 2.0
    (:`OnCompleted`
      _)
    (:`OnInterrupted`
      _))
  (`/Game/Enemies/AI/AIC_Enemy_Base.SetStateAsAttacking` _aicenemybase (`/Game/Enemies/AI/AIC_Enemy_Base.Attack Target` _aicenemybase) true))

(fn `GetCurrentHealth`
  (returns (Health :type "Float (double-precision)"))
  (return (`/Game/DamageSystem/BPC_DamageComponent.Health` (`self.BPC_DamageComponent`))))

(fn `GetIdealRange`
  (returns (AttackRadius :type "Float (double-precision)") (DefendRadius :type "Float (double-precision)"))
  (return 0.0 0.0))

(fn `getIsWieldingSword`
  (returns (SwordStatus :type Boolean))
  (return (`self.IsWieldingWeapon`)))

(fn `GetMaxHealth`
  (returns (Health :type "Float (double-precision)"))
  (return (`/Game/DamageSystem/BPC_DamageComponent.MaxHealth` (`self.BPC_DamageComponent`))))

(fn `getPatrolRoute`
  (returns (PatrolRoute :type "/Game/Enemies/AI/BP_SplineBase Object Reference"))
  (return null))

(fn `Heal`
  (params (Amount :type "Float (double-precision)"))
  (returns (NewHealth :type "Float (double-precision)"))
  (bind _newhealth (`/Game/DamageSystem/BPC_DamageComponent.Heal` (`self.BPC_DamageComponent`) Amount))
  (return _newhealth))

(fn `IsDead`
  (returns (IsDead :type Boolean))
  (return (`/Game/DamageSystem/BPC_DamageComponent.Isdead` (`self.BPC_DamageComponent`))))

(fn `SetMovementSpeed`
  (params (SpeedEnum :type "/Game/Enemies/AI/Enums/E_MovementSpeed Enum" :default "NewEnumerator0"))
  (returns (SpeedValue :type "Float (double-precision)"))
  (return 0.0))

(fn `SetVisibility`
  (`SceneComponent.SetVisibility` (`self.HealthBar`) true false))

(fn `TakeDamage`
  (params (DamageInfo :type "/Game/DamageSystem/S_DamageInfo Structure"))
  (returns (WasDamaged :type Boolean))
  (bind _wasdamaged (`/Game/DamageSystem/BPC_DamageComponent.TakeDamage` (`self.BPC_DamageComponent`) DamageInfo))
  (return _wasdamaged))

(fn `UserConstructionScript`
  (bind _bpc_damagecomponent (`self.BPC_DamageComponent`))
  (add `/Game/DamageSystem/BPC_DamageComponent.OnDeath` _bpc_damagecomponent (`|CreateDelegate` :!event `Death`))
  (add `/Game/DamageSystem/BPC_DamageComponent.OnBlocked` _bpc_damagecomponent (`|CreateDelegate` :!event `Blocked`))
  (add `/Game/DamageSystem/BPC_DamageComponent.DamageResponce` _bpc_damagecomponent (`|CreateDelegate` :!event `DamageResponce`))
  (set `/Game/DamageSystem/BPC_DamageComponent.MaxHealth` 20.0 _bpc_damagecomponent)
  (set `/Game/DamageSystem/BPC_DamageComponent.Health` 20.0 _bpc_damagecomponent))