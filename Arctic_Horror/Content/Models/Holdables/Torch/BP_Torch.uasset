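; BP_Torch is a holdable torch with a battery that drains while its spotlight is on.
; SwitchOnOff plays a sound and toggles the light, requiring minimum charge to turn on; an empty battery switches it off.
; While off, Tick recharges through holding, with FMOD winding audio, or faster through repeated taps, capped at full.
; A looping timer resets the tap count and ends fast charge; debug prints show the state.
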(event `self.ReceiveTick`
  (params (DeltaSeconds :type "Float (single-precision)"))
  (set `self.Delta Seconds` DeltaSeconds)
  (if (`self.IsTurnedOn`)
    ;[0 0 0 1 30] DRAIN BATTERY
    (if (> (`self.BatteryLife`) 0.0)
      (bind _output_get (set `self.BatteryLife` (- (`self.BatteryLife`) (* (`self.Delta Seconds`) 3.0))))
      (if (not (> _output_get 100.0))
        (`KismetSystemLibrary.PrintString` (`KismetStringLibrary.Conv_DoubleToString` (`self.BatteryLife`)) true true (struct :`G` 0.66 :`B` 1.0 :`A` 1.0) 0.1 :!label _label))
      (else
        (`self.SwitchOn/Off`)
        (`KismetSystemLibrary.PrintString` "Hello")))
    (else
      ;[0 0 0 1 30] RECHARGE
      (if (`self.FastCharge`)
        (set `self.BatteryLife` (+ (* (`self.Delta Seconds`) 10.0) (`self.BatteryLife`)))
        ;[0 0 0] STOP WHEN FULL
        (if (>= (`self.BatteryLife`) 100.0) :!label _label_2
          (set `self.BatteryLife` 100.0)
          (goto _label)
          (else
            (goto _label)))
        (elif (`self.ChargingActive`)
          (set `self.BatteryLife` (+ (* (`self.Delta Seconds`) 5.0) (`self.BatteryLife`)))
          (goto _label_2))))))

(event `TapCharge`
  (bind _fastchargecounter (`self.FastChargeCounter`))
  ;[0 0 0 1 30] Tapping to charge
  (`KismetSystemLibrary.K2_SetTimerDelegate` (delegate `StopTapCharge`) 0.6 true)
  (bind _result (`/Engine/EditorBlueprintResources/StandardMacros.IncrementInt` _fastchargecounter)
    (:`  `
      (if (> _fastchargecounter 1)
        (set `self.FastCharge` true))
      (`KismetSystemLibrary.PrintString` (`KismetStringLibrary.Conv_IntToString` _result)))))

(event `StopTapCharge`
  ;[0 0 0 1 30] Tapping to charge
  (if (`self.FastCharge`)
    (set `self.FastCharge` false)
    (`KismetSystemLibrary.PrintString` "Stopped Quick Charge" true true (struct :`R` 1.0 :`A` 1.0)))
  (set `self.FastChargeCounter` 0))

(event `ChargeActivate`
  (params (ShouldActivate :type Boolean))
  (bind _fmodcharge (`self.FMODCharge`))
  ;[0 0 0 1 30] Holding charge function
  (bind _output_get (set `self.ChargingActive` ShouldActivate))
  (if _output_get
    (`FMODAudioComponent.SetParameter` (`self.FMODCharge`) "WindingState" 1.0)
    (`FMODAudioComponent.Play` (`self.FMODCharge`))
    (else
      (`FMODAudioComponent.SetParameter` _fmodcharge "WindingState" 0.0)
      (`FMODAudioComponent.Stop` _fmodcharge))))

(fn `SwitchOn/Off`
  (`FMODAudioComponent.Play` (`self.FMODTorchon/off`))
  (if (not (`self.IsTurnedOn`))
    (if (and (not (`self.IsTurnedOn`)) (>= (`self.BatteryLife`) 10.0))
      (`SceneComponent.SetVisibility` (`self.SpotLight`) true false)
      (set `self.IsTurnedOn` true))
    (else
      (`SceneComponent.SetVisibility` (`self.SpotLight`) false false)
      (set `self.IsTurnedOn` false))))

(fn `UserConstructionScript`)