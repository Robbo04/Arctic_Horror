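; Actor component that manages health, healing, damage and death for its owner.
; TakeDamage reads a damage info struct and uses the CanBeDamaged macro to route hits to blocked, damaged or ignored outcomes, based on invincibility, blocking and death state.
; Blocks, deaths and non-lethal damage responses are broadcast through event calls, while Heal clamps health to the maximum.
; The interrupt check in TakeDamage is present but never runs.
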(event `self.ReceiveBeginPlay`
  (set `self.Health` (`self.MaxHealth`)))

(event `self.ReceiveTick`
  (params (DeltaSeconds :type "Float (single-precision)")))

(fn `Heal`
  (params (Amount :type "Float (double-precision)"))
  (returns (NewHealth :type "Float (double-precision)"))
  (if (not (`self.Isdead`))
    (bind _output_get (set `self.Health` (`KismetMathLibrary.FClamp` (+ Amount (`self.Health`)) 0.0 (`self.MaxHealth`))))
    (return _output_get)))

(fn `TakeDamage`
  (params (DamageInfo :type "/Game/DamageSystem/S_DamageInfo Structure"))
  (returns (WasDamaged :type Boolean))
  (bind (_amount _shoulddamageinvincible _canbeblocked _damageresponse _shouldforceinterrupt) (break `/Game/DamageSystem/S_DamageInfo` DamageInfo))
  (`self.CanBeDamaged` _shoulddamageinvincible _canbeblocked
    (:`BlockedDamage`
      (`self.OnBlocked`))
    (:`DoDamage`
      (bind _output_get (set `self.Health` (- (`self.Health`) _amount)))
      (if (<= _output_get 0.0)
        (set `self.Isdead` true)
        (`self.OnDeath`)
        (else
          (`self.DamageResponce` _damageresponse)))
      (return true))
    (:`NoDamage`
      (return false))))